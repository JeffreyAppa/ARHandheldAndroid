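; AR pawn that places cubes on detected real-world geometry when the screen is touched.
; It starts an AR session on BeginPlay and stops it on EndPlay.
; On touch, it traces from the screen point for existing objects; if none is hit, it traces AR tracked geometry, excluding feature points and the ground plane.
; The first tracked result supplies the transform for spawning a BP_Cube.
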(event EventBeginPlay
  (Class|ARBlueprintLibrary|StartARSession "/Game/D_sessionConfig.D_sessionConfig"))

(event Collision|EventActorBeginOverlap
  (params (OtherActor :type Actor%20Object%20Reference)))

(event EventTick
  (params (DeltaSeconds :type Float%20%28single-precision%29)))

(event EventEndPlay
  (params (EndPlayReason :type EEndPlayReason%20Enum :default "Destroyed"))
  (Class|ARBlueprintLibrary|StopARSession))

(event Input|TouchEvents|InputTouch
  (params (Location :type Vector) (FingerIndex :type ETouchIndex%20Enum))
  (bind _returnvalue (Game|GetPlayerController 0))
  (bind (_locationx _locationy) (Class|PlayerController|GetInputTouchState _returnvalue "Touch1"))
  (bind _returnvalue_2 (Math|Vector2D|MakeVector2D _locationx _locationy))
  (bind (_worldposition _worlddirection) (Class|GameplayStatics|DeprojectScreentoWorld _returnvalue _returnvalue_2))
  (:Pressed
    ;[1 1 1] check other virtual objects
    (bind _returnvalue_3 (Collision|LineTraceForObjects _worldposition (+ _worldposition (* _worlddirection 1e+03)) (Utilities|Array|MakeArray "ObjectTypeQuery1" "ObjectTypeQuery2" "ObjectTypeQuery3" "ObjectTypeQuery4" "ObjectTypeQuery5" "ObjectTypeQuery6") false 0 "None"))
    (if (not _returnvalue_3)
      ;[1 1 1] check tracked geometry
      (bind _returnvalue_4 (Class|ARBlueprintLibrary|LineTraceTrackedObjects _returnvalue_2 false false))
      (Math|Integer|CompareInt (Utilities|Array|Length _returnvalue_4)
        (:>
          (Game|SpawnActorfromClass "/Game/BP_Cube.BP_Cube_C" (Class|ARTraceResultLibrary|GetLocaltoWorldTransform (Utilities|Array|Get(acopy) _returnvalue_4)) "Undefined" 0 0))))))

(fn ConstructionScript)